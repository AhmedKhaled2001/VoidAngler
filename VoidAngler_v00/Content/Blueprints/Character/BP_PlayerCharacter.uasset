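; Player character Blueprint for a board-riding pawn that feeds its movement state to materials and shows a crosshair.
; BeginPlay creates the crosshair widget and adds it to the viewport.
; Tick writes location and the physics controller's speed ratio to a Material Parameter Collection.
; It also writes a direction built from the board's reversed horizontal velocity, rotated 90 degrees around the board's up vector.
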(event `self.ReceiveBeginPlay`
  (bind _returnvalue (`|CreateWidget` "/Game/UI/WBP_Crosshair.WBP_Crosshair_C" (`GameplayStatics.GetPlayerController` 0)))
  (`UserWidget.AddToViewport` _returnvalue 0))

(event `self.ReceiveTick`
  (params (DeltaSeconds :type "Float (single-precision)"))
  (bind (_returnvalue_x _returnvalue_y _returnvalue_z) (`KismetMathLibrary.BreakVector` (`self.K2_GetActorLocation`)))
  (bind _boardcomponentt (`self.BoardComponentt`))
  (bind (_returnvalue_x_2 _returnvalue_y_2) (`KismetMathLibrary.BreakVector` (`SceneComponent.GetComponentVelocity` _boardcomponentt)))
  (bind (_returnvalue_x_3 _returnvalue_y_3) (`KismetMathLibrary.BreakVector` (`KismetMathLibrary.RotateAngleAxis` (`KismetMathLibrary.Normal` (* (`KismetMathLibrary.MakeVector` _returnvalue_x_2 _returnvalue_y_2) -1.0)) 90.0 (`KismetMathLibrary.Normal` (`SceneComponent.GetUpVector` _boardcomponentt)))))
  (bind _returnvalue (`KismetMathLibrary.MakeColor` _returnvalue_x_3 _returnvalue_y_3))
  (`KismetMaterialLibrary.SetVectorParameterValue` (`self.MPC`) "PlayerLocation" (`KismetMathLibrary.MakeColor` _returnvalue_x _returnvalue_y _returnvalue_z))
  (`KismetMaterialLibrary.SetScalarParameterValue` (`self.MPC`) "SpeedRatio" (`PhysicsController.CurrentSpeedRatio` (`self.PhysicsControllerr`)))
  (set `self.OldRotationVector` _returnvalue)
  (if true
    (`KismetMaterialLibrary.SetVectorParameterValue` (`self.MPC`) "PlayerDirection" _returnvalue)))

(fn `UserConstructionScript`)